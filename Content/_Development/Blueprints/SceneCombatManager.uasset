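; Scene combat manager that starts a hardcoded test combat on BeginPlay, with global time slowed and anchors placed.
; It listens for phase-end events and creates the next wave when the Opening phase finishes.
; SpawnCharacter spawns a CBP_SpawnedCharacter with its data, anchor and a reference back to the manager, adjusting around collisions.
; Tick prints the current combat phase on screen for debugging.
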(event `self.ReceiveBeginPlay`
  (`GameplayStatics.SetGlobalTimeDilation` 0.15)
  (`self.PlaceAnchors`)
  (`self.InitCombat` "/Game/_Development/GameDatas/CombatDatas/Dat_Combat_TestCombat.Dat_Combat_TestCombat")
  (add `self.OnPhaseEnded` (delegate `OnPhaseEnded_Event`)))

(event `OnPhaseEnded_Event` :!signature `self.OnPhaseEnded`
  (params (EndedCombatPhase :type "ECombatPhase Enum" :default "Opening"))
  (switch `ECombatPhase` EndedCombatPhase
    (:`Opening`
      (`self.CreateNextWave`))))

(event `self.ReceiveTick`
  (params (DeltaSeconds :type "Float (single-precision)"))
  (`KismetSystemLibrary.PrintString` (`KismetStringLibrary.Concat_StrStr` "Combat Phase: " (`|GetEnumeratorNameAsString` (`self.CurrentPhase`))) true false (struct :`R` 1.0 :`G` 0.219716 :`A` 1.0) 2.0 "state"))

(fn `SpawnCharacter`
  (params (data :type "BaseCharacterData Object Reference") (spawnTr :type "Transform Structure") (charAnchor :type "CharacterAnchor Object Reference"))
  (returns (ReturnValue :type "BaseGasCharacter Object Reference"))
  (bind _returnvalue (`|SpawnActorFromClass` "/Game/_Development/Blueprints/CBP_SpawnedCharacter.CBP_SpawnedCharacter_C" spawnTr "AdjustIfPossibleButAlwaysSpawn" "MultiplyWithRoot" null data charAnchor self null))
  (return _returnvalue))

(fn `UserConstructionScript`)