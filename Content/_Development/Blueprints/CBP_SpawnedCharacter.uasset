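; Spawned character Blueprint that reacts to changes of its assigned anchor and visualizes its anchor state.
; On BeginPlay it binds to the anchor-changed event, which tries a Dash move to the anchor when the character's data is EnemyData.
; While the anchor is valid, Tick draws a debug arrow to it and a label showing the current anchor movement type.
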(event `self.ReceiveBeginPlay`
  (add `self.OnAnchorChanged` (delegate `OnAnchorChanged_Event`)))

(event `OnAnchorChanged_Event` :!signature `self.OnAnchorChanged`
  (params (OldAnchor :type "CharacterAnchor Object Reference") (NewAnchor :type "CharacterAnchor Object Reference"))
  (if (`GameplayStatics.ObjectIsA` (`self.CharacterData`) "/Script/CodeNameKibarun.EnemyData")
    (`self.TryMoveToAnchor` "Dash")))

(event `self.ReceiveTick`
  (params (DeltaSeconds :type "Float (single-precision)"))
  (bind _returnvalue (`self.K2_GetActorLocation`))
  (bind _anchor (`self.Anchor`)
    (:`then`
      (`KismetSystemLibrary.DrawDebugArrow` _returnvalue (`SceneComponent.K2_GetComponentLocation` _anchor) 250.0 (struct :`R` 1.0 :`B` 0.518839 :`A` 1.0))
      (`KismetSystemLibrary.DrawDebugString` (+ _returnvalue (0.0 -25.0 150.0)) (`|GetEnumeratorNameAsString` (`self.CurrentAnchorMovementType`)) null (struct :`R` 1.0 :`B` 0.497933 :`A` 1.0)))
    (:`else`)))

(fn `UserConstructionScript`)